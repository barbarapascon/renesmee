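; BP_NPC is an NPC that shows a prompt widget and dialogue text while the player is nearby.
; Both start hidden in the construction script, and the Trigger overlap events toggle them when BP_Player enters or leaves.
; Interact is a stub that only casts to the player.
; Indexed-array dialogue and Narrative dialogue logic remain as disconnected nodes that never run.
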(event OnComponentBeginOverlap(Trigger)
  (params (OverlappedComponent :type Primitive%20Component%20Object%20Reference) (OtherActor :type Actor%20Object%20Reference) (OtherComp :type Primitive%20Component%20Object%20Reference) (OtherBodyIndex :type Integer) (bFromSweep :type Boolean) (SweepResult :type Hit%20Result%20Structure%20%28by%20ref%29))
  (Utilities|Casting|CastToBP_Player OtherActor)
  (Rendering|SetVisibility (Variables|Default|GetWidget) true false)
  (Rendering|SetVisibility (Variables|Default|GetDialogueText) true false))

(event OnComponentEndOverlap(Trigger)
  (params (OverlappedComponent :type Primitive%20Component%20Object%20Reference) (OtherActor :type Actor%20Object%20Reference) (OtherComp :type Primitive%20Component%20Object%20Reference) (OtherBodyIndex :type Integer))
  (Utilities|Casting|CastToBP_Player OtherActor)
  (Rendering|SetVisibility (Variables|Default|GetWidget) false false)
  (Rendering|SetVisibility (Variables|Default|GetDialogueText) false false))

(event EventInteract
  (if true
    (Utilities|Casting|CastToBP_Player (stale OnComponentBeginOverlap(Trigger) OtherActor))
    (else
      (Development|PrintString "nothin"))))

(event EventBeginPlay)

(fn ConstructionScript
  (Rendering|SetVisibility (Variables|Default|GetWidget) false false)
  (Rendering|SetVisibility (Variables|Default|GetDialogueText) false false))