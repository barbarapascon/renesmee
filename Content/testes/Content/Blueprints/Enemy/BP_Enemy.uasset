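; BP_Enemy is an enemy that spots the player and makes a short-range melee attack.
; PawnSensing sets a "HasSeenPlayer?" Blackboard flag on its AI controller when it sees BP_Player.
; AttackPlayer sphere-traces just ahead, with debug drawing, damages a hit player and updates IsAttacking.
; Interact and trigger overlaps are empty; dialogue and flipbook logic is left disconnected, and the construction script hides the dialogue widgets.
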(event OnComponentBeginOverlap(Trigger)
  (params (OverlappedComponent :type Primitive%20Component%20Object%20Reference) (OtherActor :type Actor%20Object%20Reference) (OtherComp :type Primitive%20Component%20Object%20Reference) (OtherBodyIndex :type Integer) (bFromSweep :type Boolean) (SweepResult :type Hit%20Result%20Structure%20%28by%20ref%29)))

(event OnComponentEndOverlap(Trigger)
  (params (OverlappedComponent :type Primitive%20Component%20Object%20Reference) (OtherActor :type Actor%20Object%20Reference) (OtherComp :type Primitive%20Component%20Object%20Reference) (OtherBodyIndex :type Integer)))

(event OnSeePawn(PawnSensing)
  (params (Pawn :type Pawn%20Object%20Reference))
  (Utilities|Casting|CastToBP_Player Pawn)
  (AI|Components|Blackboard|SetValueasBool (AI|GetBlackboard (AI|GetAIController self)) (Utilities|Name|MakeLiteralName "HasSeenPlayer?") true))

(event Custom|AttackPlayer
  (bind _returnvalue (Transformation|GetActorLocation))
  (bind (_outhit _returnvalue_2) (Collision|SphereTraceForObjects _returnvalue (+ _returnvalue (* (Math|Vector|GetForwardVector (Transformation|GetActorRotation)) 5e+01)) 5e+01 (Utilities|Array|MakeArray "ObjectTypeQuery3") false 0 "ForOneFrame"))
  (if _returnvalue_2
    (Utilities|Casting|CastToBP_Player (.HitActor (Collision|BreakHitResult _outhit)))
    (Variables|Default|SetIsAttacking? true)
    (Game|Damage|ApplyDamage (.HitActor (Collision|BreakHitResult _outhit)) 1.0 0 0)
    (else
      (Variables|Default|SetIsAttacking? false))))

(event EventInteract)

(fn ConstructionScript
  (Rendering|SetVisibility (Variables|Default|GetWidget) false false)
  (Rendering|SetVisibility (Variables|Default|GetDialogueText) false false))