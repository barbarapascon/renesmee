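; BR_Door is an interactable door that opens and closes through a Paper2D flipbook animation.
; A Sphere trigger shows the InteractDoor component while a BP_Player overlaps it and hides it on exit, with the component hidden at construction.
; The Interact event assigns a non-looping opening flipbook, then alternates via FlipFlop between playing it forward and in reverse, so one animation serves both directions.
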(event OnComponentBeginOverlap(Sphere)
  (params (OverlappedComponent :type Primitive%20Component%20Object%20Reference) (OtherActor :type Actor%20Object%20Reference) (OtherComp :type Primitive%20Component%20Object%20Reference) (OtherBodyIndex :type Integer) (bFromSweep :type Boolean) (SweepResult :type Hit%20Result%20Structure%20%28by%20ref%29))
  (Utilities|Casting|CastToBP_Player OtherActor)
  (Rendering|SetVisibility (Variables|Default|GetInteractDoor) true false))

(event OnComponentEndOverlap(Sphere)
  (params (OverlappedComponent :type Primitive%20Component%20Object%20Reference) (OtherActor :type Actor%20Object%20Reference) (OtherComp :type Primitive%20Component%20Object%20Reference) (OtherBodyIndex :type Integer))
  (Utilities|Casting|CastToBP_Player OtherActor)
  (Rendering|SetVisibility (Variables|Default|GetInteractDoor) false false))

(event EventBeginPlay)

(event Collision|EventActorBeginOverlap
  (params (OtherActor :type Actor%20Object%20Reference)))

(event EventTick
  (params (DeltaSeconds :type Float%20%28single-precision%29)))

(event EventInteract
  (bind _door (Variables|Default|GetDoor))
  (bind _door_2 (Variables|Default|GetDoor))
  (Components|Timeline|SetLooping _door false)
  (Sprite|SetFlipbook _door "/Game/Blueprints/Objects/FB_DoorOpen.FB_DoorOpen")
  (Utilities|FlowControl|FlipFlop
    (:A
      (Components|Timeline|PlayfromStart _door_2))
    (:B
      (Components|Timeline|ReversefromEnd _door_2))))

(fn ConstructionScript
  (Rendering|SetVisibility (Variables|Default|GetInteractDoor) false false))