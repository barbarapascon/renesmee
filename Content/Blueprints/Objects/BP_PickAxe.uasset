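; BP_PickAxe is a pickaxe pickup that the player equips in hand.
; A separate display component shows it in the world, while the construction script hides the held PickAxe component.
; Pickup destroys the display, reveals PickAxe, detaches any item already in BP_Player's Equip, stores itself there and snaps to the Hand socket on the player's Sprite.
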(event EventBeginPlay)

(event Collision|EventActorBeginOverlap
  (params (OtherActor :type Actor%20Object%20Reference)))

(event EventTick
  (params (DeltaSeconds :type Float%20%28single-precision%29)))

(event EventPickup
  (bind _returnvalue (Game|GetPlayerCharacter 0))
  (bind _defaultsceneroot (Variables|Default|GetDefaultSceneRoot))
  (bind _asbp_player (Utilities|Casting|CastToBP_Player _returnvalue))
  (Components|DestroyComponent (Variables|Default|GetDisplayPickAxe))
  (Rendering|SetVisibility (Variables|Default|GetPickAxe) true false)
  (Utilities|IsValid (Variables|/Game/Blueprints/Player/BP_Player.BP_Player_C|GetEquip (.AsBP%20Player (Utilities|Casting|CastToBP_Player (Game|GetPlayerCharacter 0))))
    (:Is%20Valid
      (Transformation|DetachFromActor (Variables|/Game/Blueprints/Player/BP_Player.BP_Player_C|GetEquip (.AsBP%20Player (Utilities|Casting|CastToBP_Player (Game|GetPlayerCharacter 0)))) "KeepRelative" "KeepRelative" "KeepRelative")
      (Transformation|SetActorLocationAndRotation (Transformation|GetWorldLocation _defaultsceneroot) (Transformation|GetWorldRotation _defaultsceneroot)))
    (:Is%20Not%20Valid
      _))
  (Variables|/Game/Blueprints/Player/BP_Player.BP_Player_C|SetEquip _asbp_player self)
  (Transformation|AttachComponentToComponent (Variables|/Script/Paper2D.PaperCharacter|GetSprite _asbp_player) "Hand" "SnapToTarget" "SnapToTarget" "KeepRelative" true))

(fn ConstructionScript
  (Rendering|SetVisibility (Variables|Default|GetPickAxe) false false))