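; Item data component that makes its owning actor a pickup for the inventory, holding an item row ID and quantity.
; Interaact passes both to the interactor's InventorySystem Pickup and destroys the owner on success.
; EventInteractt makes the same call on player 0 cast to BP_Player22, but leaves the actor in place.
; FocusTarget returns an empty string and GuardaItemm is an empty stub.
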(event Custom|EventInteractt
  (bind _asbp_player_22 (Utilities|Casting|CastToBP_Player22 (Game|GetPlayerCharacter 0)))
  (bind _sucess (Default|Pickup (Variables|/Game/Blueprints/Player/BP_Player22.BP_Player22_C|GetInventorySystem _asbp_player_22) (.RowName (Utilities|Struct|BreakDataTableRowHandle (Variables|Default|GetItemId))) (Variables|Default|GetitemQuantity)))
  (if _sucess
    _))

(event EventInteraact
  (params (interactor :type BP%20Player%2022%20Object%20Reference))
  (bind _inventorysystem (Variables|/Game/Blueprints/Player/BP_Player22.BP_Player22_C|GetInventorySystem interactor)
    (:then
      (bind _sucess (Default|Pickup _inventorysystem (Utilities|Struct|BreakDataTableRowHandle (Variables|Default|GetItemId)) (Variables|Default|GetitemQuantity)))
      (if _sucess
        (Actor|DestroyActor (Components|GetOwner))))
    (:else)))

(fn FocusTarget
  (return ""))

(fn GuardaItemm
  (return ""))