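; Base world item actor for the inventory system that can be focused and picked up.
; FocusTarget looks up the item's data table row through its BPCItemData component and returns a "Pickup {Item}" prompt with the item name.
; GuardaItemm prints a pickup message, destroys the actor and returns the item, while a separate destroyitem event destroys it after a short delay.
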(event Custom|destroy%20item
  (Utilities|FlowControl|Delay 0.1)
  (Actor|DestroyActor))

(fn ConstructionScript)

(fn FocusTarget
  (bind _bpc_itemdata (Variables|Default|GetBPC_itemData))
  (bind _itemid (Variables|/Game/Blueprints/inventory/BPC_itemData.BPC_itemData_C|GetItemId _bpc_itemdata))
  (bind (_datatable _rowname) (Utilities|Struct|BreakDataTableRowHandle _itemid))
  (bind _returnvalue (Utilities|GetDataTableRow _datatable _rowname)
    (:then
      (return (Utilities|Text|FormatText "Pickup {Item}" (Utilities|Text|ToText(Name) (.ItemName (Utilities|Struct|BreakS_itemData _returnvalue))))))))

(fn GuardaItemm
  (Development|PrintString "pegou itemmm")
  (Actor|DestroyActor)
  (return (Variables|Default|Getitem)))