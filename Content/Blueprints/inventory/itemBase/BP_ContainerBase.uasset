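; BP_ContainerBase is a base Blueprint for searchable inventory containers.
; On BeginPlay it copies its ContainerContent into the InventorySystem's ItemSlot array, then resizes that array to ContainerSize.
; FocusTarget supplies a "Search {Container}" prompt built from ContainerName, while GuardaItemm is an empty stub.
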(event EventBeginPlay
  (bind _inventorysystem (Variables|Default|GetInventorySystem))
  (Variables|/Game/Blueprints/inventory/InventorySystem.InventorySystem_C|SetitemSlot _inventorysystem (Variables|Default|GetContainerContent))
  (Utilities|Array|Resize (Variables|/Game/Blueprints/inventory/InventorySystem.InventorySystem_C|GetitemSlot _inventorysystem) (Variables|Default|GetcontainerSize)))

(fn ConstructionScript)

(fn FocusTarget
  (return (Utilities|Text|FormatText "Search {Container}" (Variables|Default|GetContainerName))))

(fn GuardaItemm
  (return ""))