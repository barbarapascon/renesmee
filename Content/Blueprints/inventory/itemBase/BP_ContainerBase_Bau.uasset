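; BP_ContainerBase_Bau is a chest ("baú") container in the inventory item set that players can open and close.
; OnInteract and UpdateContainer share one branch that flips IsOpen and plays an open or close sound at the actor's location.
; A ContainerTimeline node exists but is never executed, so the graph drives no opening animation or item logic.
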(event EventBeginPlay
  (|CallParentFunction) ; Este nó está desativado e não será chamado.\nArraste os pinos para criar funcionalidade.
)

(event EventOnInteract
  (bind _returnvalue (Transformation|GetActorLocation))
  (if (not (Variables|Default|GetisOpen))
    (Variables|Default|SetisOpen true)
    (Audio|PlaySoundatLocation "/Engine/VREditor/Sounds/UI/Dockable_Window_Open.Dockable_Window_Open" _returnvalue "0, 0, 0" 1.0 1.0 0.0 0 0 0 0)
    (else
      (Variables|Default|SetisOpen false)
      (Audio|PlaySoundatLocation "/Engine/VREditor/Sounds/UI/Dockable_Window_Close.Dockable_Window_Close" _returnvalue "0, 0, 0" 1.0 1.0 0.0 0 0 0 0))))

(event EventUpdateContainer
  (bind _returnvalue (Transformation|GetActorLocation))
  (if (not (Variables|Default|GetisOpen))
    (Variables|Default|SetisOpen true)
    (Audio|PlaySoundatLocation "/Engine/VREditor/Sounds/UI/Dockable_Window_Open.Dockable_Window_Open" _returnvalue "0, 0, 0" 1.0 1.0 0.0 0 0 0 0)
    (else
      (Variables|Default|SetisOpen false)
      (Audio|PlaySoundatLocation "/Engine/VREditor/Sounds/UI/Dockable_Window_Close.Dockable_Window_Close" _returnvalue "0, 0, 0" 1.0 1.0 0.0 0 0 0 0))))

(fn ConstructionScript
  (|CallParentFunction))