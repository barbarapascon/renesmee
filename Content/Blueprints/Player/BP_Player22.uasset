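; BP_Player22 is the player character, handling Enhanced Input movement, dialog interaction, item pickup and an M-key inventory toggle.
; Interact messages every overlapping actor, while pickup messages the first one implementing BPI_PickAxe that is not already equipped.
; Jump is faked by a Delay loop that integrates speed and growing gravity to offset the sprite's relative Y.
; Tick creates and adds a new health widget every frame.
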(event Input|EnhancedActionEvents|EnhancedInputActionIA_Move
  (params (ActionValue :type Vector%202D%20Structure) (ElapsedSeconds :type Float%20%28double-precision%29) (TriggeredSeconds :type Float%20%28double-precision%29) (InputAction :type Input%20Action%20Object%20Reference :default "/Game/Blueprints/Player/IA_Move.IA_Move"))
  (:Triggered
    (Pawn|Input|AddMovementInput "1.000000,0.000000,0.000000" (.x ActionValue) true)
    (Pawn|Input|AddMovementInput "0.000000,-1.000000,0.000000" (.y ActionValue) true)
    (Variables|Default|SetDirectionality (Math|Vector2D|MakeVector2D (.x ActionValue) (.y ActionValue))))
  (:Started
    (Variables|Default|SetIsHoldingMove? true))
  (:Completed
    (Variables|Default|SetIsHoldingMove? false)))

(event Input|EnhancedActionEvents|EnhancedInputActionIA_Jump
  (params (ActionValue :type Boolean) (ElapsedSeconds :type Float%20%28double-precision%29) (TriggeredSeconds :type Float%20%28double-precision%29) (InputAction :type Input%20Action%20Object%20Reference :default "/Game/Blueprints/Player/IA_Jump.IA_Jump"))
  (bind _flipbooktransform (Variables|Default|GetFlipbookTransform))
  (bind (_x _y _z) (Math|Vector|BreakVector _flipbooktransform))
  (:Started
    (if (not (Variables|Default|GetIsJumping))
      (Variables|Default|SetIsJumping true)
      (Variables|Default|SetZSpeed (Variables|Default|GetJumpSpeed))
      (Variables|Default|SetZvalue (+ (Variables|Default|GetZvalue) (Variables|Default|GetZSpeed)))
      (if (> (Variables|Default|GetZvalue) (Variables|Default|GetZGround)) :!label _label
        (if (> (Variables|Default|GetZSpeed) -5.0)
          (Variables|Default|SetZSpeed (+ (Variables|Default|GetZSpeed) (* (Utilities|Time|GetWorldDeltaSeconds) (Variables|Default|GetZGravidity))))
          (Variables|Default|SetZGravidity (Math|Float|Clamp(Float) (+ (Variables|Default|GetZGravidity) (Variables|Default|GetZGravidity)) -5e+01 99999.0)))
        (Variables|Default|SetZvalue (Math|Float|Clamp(Float) (+ (Variables|Default|GetZvalue) (Variables|Default|GetZSpeed)) 0.0 99999.0))
        (Transformation|SetRelativeLocation (Variables|Default|GetSprite) (Math|Vector|MakeVector _x (- _y (Variables|Default|GetZvalue)) (+ _z (* (Variables|Default|GetZvalue) 0.0))) false false)
        (Utilities|FlowControl|Delay 0.01)
        (goto _label)
        (else
          (Variables|Default|SetIsJumping false)
          (Variables|Default|SetZvalue (Variables|Default|GetZGround))
          (Variables|Default|SetZSpeed 0.0)
          (Variables|Default|SetZGravidity -0.1))))))

(event Input|EnhancedActionEvents|EnhancedInputActionIA_Pickupp
  (params (ActionValue :type Boolean) (ElapsedSeconds :type Float%20%28double-precision%29) (TriggeredSeconds :type Float%20%28double-precision%29) (InputAction :type Input%20Action%20Object%20Reference :default "/Game/Blueprints/Player/IA_Pickupp.IA_Pickupp"))
  (bind _array_element (Utilities|Array|ForEachLoopwithBreak (Collision|GetOverlappingActors 0 :!class /Script/Engine.Actor) :!label _label)
    (:LoopBody
      (if (Utilities|DoesObjectImplementInterface _array_element "/Game/Blueprints/Player/BPI_PickAxe.BPI_PickAxe_C")
        (if (!= _array_element (Variables|Default|GetEquip))
          (Class|BPIPickAxe|Pickup(Message) _array_element)
          (goto _label Break))))))

(event Input|EnhancedActionEvents|EnhancedInputActionAI_InteractDialog
  (params (ActionValue :type Boolean) (ElapsedSeconds :type Float%20%28double-precision%29) (TriggeredSeconds :type Float%20%28double-precision%29) (InputAction :type Input%20Action%20Object%20Reference :default "/Game/Blueprints/Dialog/AI_InteractDialog.AI_InteractDialog"))
  (:Started
    (for _array_element (Collision|GetOverlappingActors 0 :!class /Script/Engine.Actor)
      (if true
        (Class|BPDialogInterface|Interact(Message) _array_element)))))

(event EventBeginPlay
  (bind _asplayer_controller (Utilities|Casting|CastToPlayerController (Pawn|GetController)))
  (Input|AddMappingContext (PlayerController|LocalPlayerSubsystems|GetEnhancedInputLocalPlayerSubsystem _asplayer_controller) "/Game/Blueprints/Player/IMC_Player.IMC_Player" 0 "(bIgnoreAllPressedKeysUntilRelease=True,bForceImmediately=False,bNotifyUserSettings=False)"))

(event EventTick
  (params (DeltaSeconds :type Float%20%28single-precision%29))
  (bind _returnvalue (UserInterface|CreateWidget "/Game/Blueprints/Dialog/WB_Health.WB_Health_C" (Game|GetPlayerController 0)))
  (UserInterface|Viewport|AddtoViewport _returnvalue 0))

(event Input|KeyboardEvents|M
  (params (Key :type Key%20Structure :default "None"))
  (:Pressed
    (bind _inventorywidgetref (Variables|Default|GetinventoryWidgetRef)
      (:then
        (Widget|RemovefromParent _inventorywidgetref)
        (Variables|Default|SetinventoryWidgetRef 0))
      (:else
        (bind _returnvalue (UserInterface|CreateWidget "/Game/Blueprints/Dialog/WB_INVENTORY.WB_INVENTORY_C" (Game|GetPlayerController 0)))
        (bind _output_get (Variables|Default|SetinventoryWidgetRef _returnvalue))
        (UserInterface|Viewport|AddtoViewport _output_get 0)))))

(fn ConstructionScript)

(fn GettingOverlappingInteractions
  (params (Box :type Primitive%20Component%20Object%20Reference))
  (for _array_element (Collision|GetOverlappingActors Box "/Script/Engine.Actor" :!class /Script/Engine.PrimitiveComponent)
    (if (Class|KismetSystemLibrary|DoesClassImplementInterface (Utilities|GetClass _array_element) "/Game/Blueprints/Dialog/BP_DialogInterface.BP_DialogInterface_C")
      (return _array_element true)))
  (return 0 false))