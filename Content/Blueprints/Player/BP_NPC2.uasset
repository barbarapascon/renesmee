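; BP_NPC2 is an interactable NPC that shows dialog one line at a time.
; Interact advances DialogIndex, writes that Dialog entry into a lazily created WB_Dialog, and removes it past the last line, without resetting the index.
; A hidden Trigger toggles the Widget as BP_Player enters or leaves.
; A helper function, unused here, finds the first overlapping actor implementing BP_DialogInterface.
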(event OnComponentBeginOverlap(trigger)
  (params (OverlappedComponent :type Primitive%20Component%20Object%20Reference) (OtherActor :type Actor%20Object%20Reference) (OtherComp :type Primitive%20Component%20Object%20Reference) (OtherBodyIndex :type Integer) (bFromSweep :type Boolean) (SweepResult :type Hit%20Result%20Structure%20%28by%20ref%29))
  (Utilities|Casting|CastToBP_Player OtherActor)
  (Rendering|SetVisibility (Variables|Default|GetWidget) true false))

(event OnComponentEndOverlap(trigger)
  (params (OverlappedComponent :type Primitive%20Component%20Object%20Reference) (OtherActor :type Actor%20Object%20Reference) (OtherComp :type Primitive%20Component%20Object%20Reference) (OtherBodyIndex :type Integer))
  (Utilities|Casting|CastToBP_Player OtherActor)
  (Rendering|SetVisibility (Variables|Default|GetWidget) false false))

(event EventInteract
  (Math|Integer|IncrementInt (Variables|Default|GetDialogIndex)
    (:%20%20
      (if (< (Variables|Default|GetDialogIndex) (Utilities|Array|Length (Variables|Default|GetDialog)))
        (Variables|Default|Getui
          (:then
            _)
          (:else
            (bind _returnvalue (UserInterface|CreateWidget "/Game/Blueprints/Dialog/WB_Dialog.WB_Dialog_C" (Game|GetPlayerController 0)))
            (bind _output_get (Variables|Default|Setui _returnvalue))
            (UserInterface|Viewport|AddtoViewport _output_get 0)))
        (Rendering|Components|TextRender|SetText (Variables|/Game/Blueprints/Dialog/WB_Dialog.WB_Dialog_C|Gettxt_dialog (Variables|Default|Getui)) (Utilities|Text|ToText(String) (Utilities|Array|Get(acopy) (Variables|Default|GetDialog) (Variables|Default|GetDialogIndex))))
        (else
          (bind _ui (Variables|Default|Getui)
            (:then
              (Widget|RemovefromParent _ui))
            (:else)))))))

(fn ConstructionScript
  (Rendering|SetVisibility (Variables|Default|Gettrigger) false false))

(fn GettingOverlappingInteractions
  (params (Box :type Primitive%20Component%20Object%20Reference))
  (for _array_element (Collision|GetOverlappingActors Box "/Script/Engine.Actor" :!class /Script/Engine.PrimitiveComponent)
    (if (Class|KismetSystemLibrary|DoesClassImplementInterface (Utilities|GetClass _array_element) "/Game/Blueprints/Dialog/BP_DialogInterface.BP_DialogInterface_C")
      (return _array_element true)))
  (return 0 false))