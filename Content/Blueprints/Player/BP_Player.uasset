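; Player Blueprint for a sprite-based character that moves, jumps and triggers dialog interactions through Enhanced Input.
; Movement input sets a directionality vector and pushes a Box ahead of the character.
; Jumping is faked by a Delay loop that integrates custom height and gravity, offsetting Sprite and Sombra along relative Y.
; Interact messages every overlapping actor; the interface-filtered look-at logic is left unwired.
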(event Input|EnhancedActionEvents|EnhancedInputActionIA_Move
  (params (ActionValue :type Vector%202D%20Structure) (ElapsedSeconds :type Float%20%28double-precision%29) (TriggeredSeconds :type Float%20%28double-precision%29) (InputAction :type Input%20Action%20Object%20Reference :default "/Game/Blueprints/Player/IA_Move.IA_Move"))
  (bind _returnvalue (Class|Pawn|GetLastMovementInputVector))
  (:Triggered
    (Pawn|Input|AddMovementInput "1.000000,0.000000,0.000000" (.x ActionValue) false)
    (Pawn|Input|AddMovementInput "0.000000,-1.000000,0.000000" (.y ActionValue) false)
    (Variables|Default|SetDirectionality (Math|Vector2D|MakeVector2D (.x ActionValue) (.y ActionValue)))
    (Transformation|SetRelativeLocation (Variables|Default|GetBox) (* (Math|Vector|MakeVector (.x _returnvalue) (.y _returnvalue) (.z _returnvalue)) 5e+01) false false))
  (:Started
    (Variables|Default|SetIsHoldingMove? true))
  (:Completed
    (Variables|Default|SetIsHoldingMove? false)))

(event Input|EnhancedActionEvents|EnhancedInputActionIA_Jump
  (params (ActionValue :type Boolean) (ElapsedSeconds :type Float%20%28double-precision%29) (TriggeredSeconds :type Float%20%28double-precision%29) (InputAction :type Input%20Action%20Object%20Reference :default "/Game/Blueprints/Player/IA_Jump.IA_Jump"))
  (bind _flipbooktransform (Variables|Default|GetFlipbookTransform))
  (bind (_x _y _z) (Math|Vector|BreakVector _flipbooktransform))
  (:Started
    (if (not (Variables|Default|GetIsJumping))
      (Variables|Default|SetIsJumping true)
      (Variables|Default|SetZSpeed (Variables|Default|GetJumpSpeed))
      (Variables|Default|SetZvalue (+ (Variables|Default|GetZvalue) (Variables|Default|GetZSpeed)))
      (if (> (Variables|Default|GetZvalue) (Variables|Default|GetZGround)) :!label _label
        (if (> (Variables|Default|GetZSpeed) -5.0)
          (Variables|Default|SetZSpeed (+ (Variables|Default|GetZSpeed) (* (Utilities|Time|GetWorldDeltaSeconds) (Variables|Default|GetZGravidity))))
          (Variables|Default|SetZGravidity (Math|Float|Clamp(Float) (+ (Variables|Default|GetZGravidity) (Variables|Default|GetZGravidity)) -5e+01 99999.0)))
        (Variables|Default|SetZvalue (Math|Float|Clamp(Float) (+ (Variables|Default|GetZvalue) (Variables|Default|GetZSpeed)) 0.0 99999.0))
        (Transformation|SetRelativeLocation (Variables|Default|GetSprite) (Math|Vector|MakeVector _x (- _y (Variables|Default|GetZvalue)) (+ _z (* (Variables|Default|GetZvalue) 0.0))) false false)
        (Utilities|FlowControl|Delay 0.01)
        (goto _label)
        (else
          (Variables|Default|SetIsJumping false)
          (Variables|Default|SetZvalue (Variables|Default|GetZGround))
          (Variables|Default|SetZSpeed 0.0)
          (Variables|Default|SetZGravidity -0.1))))))

(event Input|EnhancedActionEvents|EnhancedInputActionAI_InteractDialog
  (params (ActionValue :type Boolean) (ElapsedSeconds :type Float%20%28double-precision%29) (TriggeredSeconds :type Float%20%28double-precision%29) (InputAction :type Input%20Action%20Object%20Reference :default "/Game/Blueprints/Dialog/AI_InteractDialog.AI_InteractDialog"))
  (:Started
    (for _array_element (Collision|GetOverlappingActors 0 :!class /Script/Engine.Actor)
      (if true
        (Class|BPDialogInterface|Interact(Message) _array_element)))))

(event EventBeginPlay
  (bind _asplayer_controller (Utilities|Casting|CastToPlayerController (Pawn|GetController)))
  (Input|AddMappingContext (PlayerController|LocalPlayerSubsystems|GetEnhancedInputLocalPlayerSubsystem _asplayer_controller) "/Game/Blueprints/Player/IMC_Player.IMC_Player" 0 "(bIgnoreAllPressedKeysUntilRelease=True,bForceImmediately=False,bNotifyUserSettings=False)"))

(event Collision|EventActorBeginOverlap
  (params (OtherActor :type Actor%20Object%20Reference)))

(event EventTick
  (params (DeltaSeconds :type Float%20%28single-precision%29)))

(fn ConstructionScript)

(fn GettingOverlappingInteractions
  (params (Box :type Primitive%20Component%20Object%20Reference))
  (for _array_element (Collision|GetOverlappingActors Box "/Script/Engine.Actor" :!class /Script/Engine.PrimitiveComponent)
    (if (Class|KismetSystemLibrary|DoesClassImplementInterface (Utilities|GetClass _array_element) "/Game/Blueprints/Dialog/BP_DialogInterface.BP_DialogInterface_C")
      (return _array_element true)))
  (return 0 false))